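; Rendering Blueprint function that packs the world positions of the level's light components into a texture for material use.
; It scans all actors for light components, builds a vector array with the entry count prepended, and prints and draws debug spheres per light.
; The array creates or updates a generated texture, set on a new M_BaseUnlit dynamic material that it returns.
; The render target is cleared and resized but never drawn to.
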(fn UpdateLightArrays
  (bind _lightpositionarray (LocalVariables|GetLightPositionArray))
  (bind _lightpositionarray_2 (LocalVariables|GetLightPositionArray))
  (bind _returnvalue (Utilities|Array|Length _lightpositionarray_2))
  (bind _returnvalue_2 (Utilities|Array|Length _lightpositionarray))
  (Utilities|Array|Clear (LocalVariables|GetLightPositionArray))
  (bind _returnvalue_3 (Rendering|Material|CreateDynamicMaterialInstance 0 "/Game/PGC/Tests/M_BaseUnlit.M_BaseUnlit" "None" :!class /Script/Engine.KismetMaterialLibrary))
  (LocalVariables|SetDynamicTexture _returnvalue_3)
  (bind _outactors (Actor|GetAllActorsOfClass 0 "/Script/Engine.Actor"))
  (for _array_element _outactors
    (for _array_element_2 (Actor|GetComponentsByClass _array_element "/Script/Engine.LightComponentBase")
      (bind _returnvalue_4 (Utilities|Array|Add (LocalVariables|GetLightPositionArray) (Math|Vector4|MakeVector4 (.x (Transformation|GetWorldLocation _array_element_2)) (.y (Transformation|GetWorldLocation _array_element_2)) (.z (Transformation|GetWorldLocation _array_element_2)) 1.0)))
      ;[1 1 1] Debug
      (Development|PrintString 0 (Utilities|String|ToString(Text) (Utilities|Text|FormatText "Vector4[{pos}]: ({a}, {b}, {c}, {d})" _returnvalue_4 (.x (Utilities|Array|Get(acopy) (LocalVariables|GetLightPositionArray) _returnvalue_4)) (.y (Utilities|Array|Get(acopy) (LocalVariables|GetLightPositionArray) _returnvalue_4)) (.z (Utilities|Array|Get(acopy) (LocalVariables|GetLightPositionArray) _returnvalue_4)) (.w (Utilities|Array|Get(acopy) (LocalVariables|GetLightPositionArray) _returnvalue_4)))) true true "(R=1.000000,G=0.781971,B=0.000000,A=1.000000)" 1e+02)
      (Rendering|Debug|DrawDebugSphere 0 (Transformation|GetWorldLocation _array_element_2) 1e+01 12 "(R=1.000000,G=0.363357,B=0.000000,A=1.000000)" 5e+01 1.0)))
  ;[1 0 0] Array size information (red channel at vector index 0)
  (Utilities|Array|Insert (LocalVariables|GetLightPositionArray) (Math|Vector4|MakeVector4 (Math|Conversions|ToFloat(Integer) (Utilities|Array|Length (LocalVariables|GetLightPositionArray))) 0.0 0.0 0.0))
  (Rendering|ClearRenderTarget2D 0 (LocalVariables|GetRenderTarget) "(R=0.000000,G=0.000000,B=0.000000,A=0.000000)")
  (if (!= (Variables|/Script/Engine.TextureRenderTarget2D|GetSizeX (LocalVariables|GetRenderTarget)) _returnvalue_2)
    (Rendering|ResizeRenderTarget2D (LocalVariables|GetRenderTarget) _returnvalue_2 1))
  (LocalVariables|GetGeneratedArray
    (:then
      (bind _returnvalue_5 (Class|MaterialArrayUtilities|UpdateTexturefromVector (LocalVariables|GetLightPositionArray) _returnvalue (LocalVariables|GetGeneratedArray)))
      (LocalVariables|SetGeneratedArray _returnvalue_5))
    (:else
      (bind _returnvalue_6 (Class|MaterialArrayUtilities|CreateTexturefromVector (LocalVariables|GetLightPositionArray) _returnvalue))
      (LocalVariables|SetGeneratedArray _returnvalue_6)))
  (Rendering|Material|SetTextureParameterValue (LocalVariables|GetDynamicTexture) "texture" (LocalVariables|GetGeneratedArray))
  (return (LocalVariables|GetDynamicTexture)))