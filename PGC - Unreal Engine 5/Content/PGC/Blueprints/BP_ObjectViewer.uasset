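; Interactive object viewer actor that shows a mesh through a SceneCapture2D and the W_ObjectRender widget, hiding it from the main view with Owner No See.
; Construction scales and centres the mesh within Cube bounds and applies a dynamic M_Phong material to every slot.
; Mouse input rotates Cube and smoothly zooms via spring arm length or ortho width, per projection type.
; Keys reset rotation or zoom, or refresh the material through UpdateLightArrays.
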(event EventBeginPlay
  ;[0 0 0] Como esta classe não deriva de pawn, é necessário que habilitemos o suporte a inputs.
  (Input|EnableInput (Game|GetPlayerController 0))
  ;[0 0 0] Façamos agora o oposto, desligando os inputs do pawn gerado automaticamente pelo level. Como não o utilizaremos, desligamos os inputs para evitar qualquer tipo de conflito de teclas ou movimento desnecessário na tela.
  (Input|DisableInput (Game|Player|GetPlayerPawn 0) (Game|GetPlayerController 0))
  ;[0 0 0] Se o "owner" deste objeto for o pawn, marcar "owner no see" fará com que o objeto não apareça no mundo para o "pawn". Queremos isso para que apenas o scene capture possa visualizar por meio do material gerado (imagem que vemos na interface).
  (Rendering|SetActorHiddenInGame (Game|Player|GetPlayerPawn 0) true)
  (Actor|SetOwner (Game|Player|GetPlayerPawn 0))
  (Class|PrimitiveComponent|SetOwnerNoSee (Variables|Default|GetMesh) true)
  (Variables|/Script/Engine.PlayerController|SetbShowMouseCursor (Game|GetPlayerController 0) true)
  (bind _returnvalue (UserInterface|CreateWidget "/Game/PGC/Widgets/W_ObjectRender.W_ObjectRender_C" 0 self))
  (UserInterface|Viewport|AddtoViewport _returnvalue 0))

(event EventTick
  (params (DeltaSeconds :type Float%20%28single-precision%29))
  (|Zoom DeltaSeconds))

(event Input|KeyboardEvents|2
  (params (Key :type Key%20Structure :default "None"))
  ;[1 1 1] Reset zoom
  (:Pressed
    (Variables|Default|SetCurrentTargetLength (Variables|Default|GetDefaultArmLength))
    (Variables|Default|SetCurrentOrthoWidth (Variables|Default|GetDefaultOrthoWidth))))

(event Input|KeyboardEvents|1
  (params (Key :type Key%20Structure :default "None"))
  ;[1 1 1] Reset rotation
  (:Pressed
    (Transformation|SetWorldRotation (Variables|Default|GetCube) (Variables|Default|GetDefaultWorldRotation) false true)))

(event Input|KeyboardEvents|CCedille
  (params (Key :type Key%20Structure :default "None"))
  (:Pressed
    (bind _dynamictexture1 (CallFunction|UpdateLightArrays))
    (CallFunction|UpdateMaterial _dynamictexture1)))

(event Input|MouseEvents|Mouse2D
  (params (AxisValue :type Vector :default "0, 0, 0"))
  ;[1 1 1] Object rotation
  (Transformation|AddWorldRotation (Variables|Default|GetCube) (Math|Rotator|MakeRotator (* (.y AxisValue) -1.0) 0.0 (* (.x AxisValue) -1.0)) false true))

(fn ConstructionScript
  ;[1 1 1] Define o valor padrão inicial do spring arm length e ortho width.
  (bind _output_get (Variables|Default|SetCurrentTargetLength (Variables|/Script/Engine.SpringArmComponent|GetTargetArmLength (Variables|Default|GetSpringArm))))
  (Variables|Default|SetDefaultArmLength _output_get)
  (bind _output_get_2 (Variables|Default|SetCurrentOrthoWidth (Variables|/Script/Engine.SceneCaptureComponent2D|GetOrthoWidth (Variables|Default|GetSceneCapture2D))))
  (Variables|Default|SetDefaultOrthoWidth _output_get_2)
  (Variables|Default|SetDefaultWorldRotation (Transformation|GetWorldRotation (Variables|Default|GetCube)))
  (CallFunction|UpdateScale)
  (bind _returnvalue (Rendering|Material|CreateDynamicMaterialInstance "/Game/PGC/Materials/M_Phong.M_Phong" "None" "None" :!class /Script/Engine.KismetMaterialLibrary))
  (bind _output_get_3 (Variables|Default|SetCurrentMaterial _returnvalue))
  (CallFunction|UpdateMaterial _output_get_3))

(fn UpdateScale
  (bind _mesh (Variables|Default|GetMesh))
  (bind _cube (Variables|Default|GetCube))
  (bind _mesh_2 (Variables|Default|GetMesh))
  (bind (_origin _boxextent) (Collision|GetComponentBounds _mesh))
  (bind (_origin_2 _boxextent_2) (Collision|GetComponentBounds _cube))
  (Transformation|ResetRelativeTransform (Variables|Default|GetMesh))
  (Transformation|SetRelativeScale3D _mesh_2 (Math|Conversions|ToVector(Float) (Class|KismetMathLibrary|GetMinElement (/ _boxextent_2 _boxextent))))
  (Transformation|SetRelativeLocation _mesh_2 (- _origin_2 _origin) false false))

(fn UpdateMesh
  (params (NewMesh :type Static%20Mesh%20Object%20Reference))
  (Components|StaticMesh|SetStaticMesh (Variables|Default|GetMesh) NewMesh)
  (CallFunction|UpdateScale)
  (CallFunction|UpdateMaterial (Variables|Default|GetCurrentMaterial)))

(fn UpdateMaterial
  (params (CurrentMaterial :type Material%20Instance%20Dynamic%20Object%20Reference))
  (bind _output_get (Variables|Default|SetCurrentMaterial CurrentMaterial))
  (for _index (range 0 (- (Rendering|Material|GetNumMaterials (Variables|Default|GetMesh)) 1))
    (Rendering|Material|SetMaterial (Variables|Default|GetMesh) _index _output_get)))

(event Input|MouseEvents|MouseWheelAxis
  (params (AxisValue :type Float%20%28single-precision%29))
  ;[0 0 0] Zoom in/out
  (switch int (Math|Conversions|ToInteger(Byte) (Variables|/Script/Engine.SceneCaptureComponent2D|GetProjectionType (Variables|Default|GetSceneCapture2D)))
    (:0
      (Variables|Default|SetCurrentTargetLength (+ (Variables|Default|GetCurrentTargetLength) (* AxisValue -1.0 (Variables|Default|GetZoomSensitivity)))))
    (:1
      (Variables|Default|SetCurrentOrthoWidth (+ (Variables|/Script/Engine.SceneCaptureComponent2D|GetOrthoWidth (Variables|Default|GetSceneCapture2D)) (* AxisValue -1.0 (Variables|Default|GetZoomSensitivity)))))))