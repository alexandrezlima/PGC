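; BP_RoughnessVsMetallic is an actor that builds a calibration-style grid of meshes comparing material roughness against metallic.
; Its construction script spawns an 11x11 grid of static mesh components, raising roughness along X and metallic along Z.
; Each mesh gets a dynamic instance of either M_PBR or M_BaseColor, chosen by MaterialType.
; A SceneCaptureComponent2D captures the scene once the grid is built, and the event graph is unused.
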(event EventBeginPlay)

(event Collision|EventActorBeginOverlap
  (params (OtherActor :type Actor%20Object%20Reference)))

(event EventTick
  (params (DeltaSeconds :type Float%20%28single-precision%29)))

(fn ConstructionScript
  (for _index (range 0 10)
    (for _index_2 (range 0 10)
      (bind _returnvalue (AddComponent|AddStaticMeshComponent false (Math|Transform|MakeTransform (Math|Vector|MakeVector (Math|Conversions|ToFloat(Integer) (* _index_2 105)) 0.0 (Math|Conversions|ToFloat(Integer) (* _index 105))))))
      (bind _returnvalue_2 (Rendering|Material|CreateDynamicMaterialInstance (Utilities|Select :Index (Variables|Default|GetMaterialType) :Option%200 "/Game/PGC/Materials/M_PBR.M_PBR" :Option%201 "/Game/PGC/Tests/M_BaseColor.M_BaseColor") "None" "None" :!class /Script/Engine.KismetMaterialLibrary))
      (Rendering|Material|SetMaterial _returnvalue 0 _returnvalue_2)
      (Rendering|Material|SetScalarParameterValue _returnvalue_2 "Roughness" (/ _index_2 1e+01) :!class /Script/Engine.MaterialInstanceDynamic)
      (Rendering|Material|SetScalarParameterValue _returnvalue_2 "Metallic" (/ _index 1e+01) :!class /Script/Engine.MaterialInstanceDynamic)))
  (Rendering|SceneCapture|CaptureScene (Variables|Default|GetSceneCaptureComponent2D) :!class /Script/Engine.SceneCaptureComponent2D))